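; Key3BP is a key pickup that sets HasKey3 on the FirstPersonCharacter and then destroys itself.
; Box overlap by the character enables input and opens a gate, so pressing Interact only collects the key while in range; leaving reverses both.
; The prompt widget toggles on begin and end overlap before the character cast, so any overlapping actor shows or hides it.
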(event OnComponentBeginOverlap(Box)
  (params (OverlappedComponent :type Primitive%20Component%20Object%20Reference) (OtherActor :type Actor%20Object%20Reference) (OtherComp :type Primitive%20Component%20Object%20Reference) (OtherBodyIndex :type Integer) (bFromSweep :type Boolean) (SweepResult :type Hit%20Result%20Structure%20%28by%20ref%29))
  ;[1 1 1] Interactions
  (Utilities|FlowControl|Sequence
    (:then_0
      (Development|SetHiddeninGame (Variables|Default|GetWidget) false false))
    (:then_1
      (bind _asfirst_person_character_bp (Utilities|Casting|CastToFirstPersonCharacter OtherActor))
      (Input|EnableInput (Game|GetPlayerController 0))
      (Utilities|FlowControl|Gate true) ; enters at Open
    )))

(event OnComponentEndOverlap(Box)
  (params (OverlappedComponent :type Primitive%20Component%20Object%20Reference) (OtherActor :type Actor%20Object%20Reference) (OtherComp :type Primitive%20Component%20Object%20Reference) (OtherBodyIndex :type Integer))
  ;[1 1 1] Interactions
  (Utilities|FlowControl|Sequence
    (:then_0
      (Development|SetHiddeninGame (Variables|Default|GetWidget) true false))
    (:then_1
      (Utilities|Casting|CastToFirstPersonCharacter OtherActor)
      (Input|DisableInput (Game|GetPlayerController 0))
      (Utilities|FlowControl|Gate true) ; enters at Close
    )))

(event Input|ActionEvents|InputActionInteract
  (params (Key :type Key%20Structure))
  ;[1 1 1] Interactions
  (:Pressed
    (Utilities|FlowControl|Gate true
      (:Exit
        (Variables|/Game/FirstPersonCPP/Blueprints/FirstPersonCharacter.FirstPersonCharacter_C|SethasKey3 (stale OnComponentBeginOverlap(Box) _asfirst_person_character_bp) true)
        (Actor|DestroyActor)))))

(fn ConstructionScript)