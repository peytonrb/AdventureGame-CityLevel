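; Ring pickup actor that ends the game with a win when the player interacts with it.
; Box overlap shows or hides a prompt widget and, for the FirstPersonCharacter, toggles actor input and a gate.
; Pressing Interact while the gate is open creates the WinGameWidget, shows the mouse cursor, pauses the game and destroys the actor.
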(event OnComponentBeginOverlap(Box)
  (params (OverlappedComponent :type Primitive%20Component%20Object%20Reference) (OtherActor :type Actor%20Object%20Reference) (OtherComp :type Primitive%20Component%20Object%20Reference) (OtherBodyIndex :type Integer) (bFromSweep :type Boolean) (SweepResult :type Hit%20Result%20Structure%20%28by%20ref%29))
  ;[1 1 1] Interactions
  (Utilities|FlowControl|Sequence
    (:then_0
      (Development|SetHiddeninGame (Variables|Default|GetWidget) false false))
    (:then_1
      (Utilities|Casting|CastToFirstPersonCharacter OtherActor)
      (Input|EnableInput (Game|GetPlayerController 0))
      (Utilities|FlowControl|Gate true) ; enters at Open
    )))

(event OnComponentEndOverlap(Box)
  (params (OverlappedComponent :type Primitive%20Component%20Object%20Reference) (OtherActor :type Actor%20Object%20Reference) (OtherComp :type Primitive%20Component%20Object%20Reference) (OtherBodyIndex :type Integer))
  ;[1 1 1] Interactions
  (Utilities|FlowControl|Sequence
    (:then_0
      (Development|SetHiddeninGame (Variables|Default|GetWidget) true false))
    (:then_1
      (Utilities|Casting|CastToFirstPersonCharacter OtherActor)
      (Input|DisableInput (Game|GetPlayerController 0))
      (Utilities|FlowControl|Gate true) ; enters at Close
    )))

(event Input|ActionEvents|InputActionInteract
  (params (Key :type Key%20Structure))
  ;[1 1 1] Interactions
  (:Pressed
    (Utilities|FlowControl|Gate true
      (:Exit
        ;[1 1 1] Game End
        (bind _returnvalue (UserInterface|CreateWidget "/Game/WinLoseUI/WinGameWidget.WinGameWidget_C"))
        (UserInterface|Viewport|AddtoViewport _returnvalue 0)
        (Variables|/Script/Engine.PlayerController|SetbShowMouseCursor (Game|GetPlayerController 0) true)
        (Game|SetGamePaused true)
        (Actor|DestroyActor)))))

(fn ConstructionScript)